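; BP_CharBase is the client controller for a Minesweeper-style game played over a WebSocket, creating the WBP_Game board at BeginPlay.
; It connects through BP_MyTestGameInstance and parses each "map:" message into cell characters, inferring row width from the first non-leading separator via a resettable DoOnce.
; The board widget receives the filtered cells, showing a loss if "*" appears, or a win without updating when no "□" remains.
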(event Custom|RefreshMap
  (params (Nessage :type String))
  (bind _rights (Utilities|String|Split Nessage "map:"))
  (bind _returnvalue (Utilities|String|GetCharacterArrayfromString _rights))
  (if (Utilities|String|Contains Nessage "map")
    (Utilities|Array|Clear (Variables|Default|GetFilteredArray))
    (if (Utilities|Array|ContainsItem _returnvalue "□")
      (for (_array_element _array_index) _returnvalue
        (if (and (Math|Boolean|ORBoolean (Utilities|Enum|Equal(Enum) _array_element "□") (Class|KismetStringLibrary|IsNumeric _array_element) (Utilities|Enum|Equal(Enum) _array_element "*")) (not (Utilities|Array|IsEmpty _array_element)))
          (Utilities|Array|Add (Variables|Default|GetFilteredArray) _array_element)
          (elif (!= _array_index 0)
            (Utilities|FlowControl|DoOnce false
              (:Completed
                (Variables|Default|SetElemNemInRow (- _array_index 1)))))))
      (CallFunction|Reset)
      (Default|Update (Variables|Default|GetBoardWidget) (Variables|Default|GetFilteredArray) (Variables|Default|GetElemNemInRow))
      (if (Utilities|Array|ContainsItem _returnvalue "*")
        (Default|PlayMessage (Variables|Default|GetBoardWidget) "You losed!"))
      (else
        (Default|PlayMessage (Variables|Default|GetBoardWidget) "You Win!")))))

(event Custom|Reset
  (Utilities|FlowControl|DoOnce false) ; enters at Reset
)

(event Custom|CreateBoard
  (bind _returnvalue (UserInterface|CreateWidget "/Game/Project/WBP_Game.WBP_Game_C"))
  (bind _output_get (Variables|Default|SetBoardWidget _returnvalue))
  (UserInterface|Viewport|AddtoViewport _output_get 0))

(event EventBeginPlay
  (bind _asbp_my_test_game_instance (Utilities|Casting|CastToBP_MyTestGameInstance (Game|GetGameInstance)))
  (Class|MyTestGameInstance|ConnecttoWS _asbp_my_test_game_instance)
  (EventDispatchers|BindEventtoOnMessageRecieved _asbp_my_test_game_instance (delegate Custom|RefreshMap))
  (CallFunction|CreateBoard))

(fn ConstructionScript)